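; Car component for gravity engines that rotate the owning Pawn_ChaosCar for a limited power time, followed by a cooldown.
; While active, Tick adds angular velocity to the mesh from the forward/right input axes, using a separate power value during nitro.
; BeginPlay spawns four directional particle emitters and an attached sound.
; DoOnce gates switch particles and fire direction events as input starts or stops; activation and shutdown play sounds, and shutdown resets effects.
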(event `self.ReceiveBeginPlay`
  (bind (_engineparticle _attackpointname _particletransform) (break `/Game/Interaction/Blueprints/Pawn/Car/Components/Struct_GE_Particle` (`BlueprintMapLibrary.Map_Find` (`self.GravityEnginesParticles`) "Left")))
  (bind (_engineparticle_2 _attackpointname_2 _particletransform_2) (break `/Game/Interaction/Blueprints/Pawn/Car/Components/Struct_GE_Particle` (`BlueprintMapLibrary.Map_Find` (`self.GravityEnginesParticles`) "Backward")))
  (bind ((`EngineParticle_2_C88F0C694E9D841B1F643E85064A3E54` _engineparticle_3) (`AttackPointName_5_40B3EF8F4807AF72D80FADB772EBF353` _attackpointname_3)) (break `/Game/Interaction/Blueprints/Pawn/Car/Components/Struct_GE_Particle` (`BlueprintMapLibrary.Map_Find` (`self.GravityEnginesParticles`) "Forward")))
  (bind (_engineparticle_4 _attackpointname_4 _particletransform_3) (break `/Game/Interaction/Blueprints/Pawn/Car/Components/Struct_GE_Particle` (`BlueprintMapLibrary.Map_Find` (`self.GravityEnginesParticles`) "Right")))
  (bind _aspawn_chaos_car (cast `/Game/Interaction/Blueprints/Pawn/Car/Pawn_ChaosCar` (`self.GetOwner`))
    (:`then`
      (set `self.Car` _aspawn_chaos_car)
      (bind _returnvalue (`GameplayStatics.SpawnEmitterAttached` _engineparticle_3 (`WheeledVehiclePawn.Mesh` (`self.Car`)) _attackpointname_3 (0.0 0.0 0.0) (struct) (1.0 1.0 1.0) "KeepRelativeOffset" false))
      (bind _output_get (set `self.Particle_Forward` _returnvalue))
      (`self.SetActive` _output_get false false)
      (bind _returnvalue_2 (`GameplayStatics.SpawnEmitterAttached` _engineparticle_4 (`WheeledVehiclePawn.Mesh` (`self.Car`)) _attackpointname_4 (.location _particletransform_3) (.rotation _particletransform_3) (.scale _particletransform_3) "KeepRelativeOffset" false))
      (bind _output_get_2 (set `self.Particle_Right` _returnvalue_2))
      (`self.SetActive` _output_get_2 false false)
      (bind _returnvalue_3 (`GameplayStatics.SpawnEmitterAttached` _engineparticle_2 (`WheeledVehiclePawn.Mesh` (`self.Car`)) _attackpointname_2 (.location _particletransform_2) (.rotation _particletransform_2) (.scale _particletransform_2) "KeepRelativeOffset" false))
      (bind _output_get_3 (set `self.Particle_Backward` _returnvalue_3))
      (`self.SetActive` _output_get_3 false false)
      (bind _returnvalue_4 (`GameplayStatics.SpawnEmitterAttached` _engineparticle (`WheeledVehiclePawn.Mesh` (`self.Car`)) _attackpointname (.location _particletransform) (.rotation _particletransform) (.scale _particletransform) "KeepRelativeOffset" false))
      (bind _output_get_4 (set `self.Particle_Left` _returnvalue_4))
      (`self.SetActive` _output_get_4 false false)
      (bind _returnvalue_5 (`GameplayStatics.SpawnSoundAttached` (`self.EngineStart_Sound`) (`WheeledVehiclePawn.Mesh` (`self.Car`)) "None" (0.0 0.0 0.0) (struct) "KeepRelativeOffset" false 1.0 1.0 0.0 null null false))
      (bind _output_get_5 (set `self.Sound` _returnvalue_5))
      (`AudioComponent.Stop` _output_get_5))
    (:`CastFailed`
      (`KismetSystemLibrary.PrintString` "(Impulse System) Owner actor is not a car"))))

(event `GravityEngineActivate`
  (params (Active :type Boolean))
  ;[1 1 1] Activate/Deactivate GravityEngines
  (if (`self.IsCooldown`)
    (`|ExecutionSequence`
      (:`then_0`
        (goto _label :!via `Reset`))
      (:`then_1`
        (goto _label_2 :!via `Reset`)))
    (elif Active
      (`|ExecutionSequence`
        (:`then_0`
          (`/Engine/EditorBlueprintResources/StandardMacros.DoOnce` false :!label _label
            (:`Completed`
              (`self.SetComponentTickEnabled` true)
              (set `self.GravityEnginesActive` true)
              (`self.PlayGravityEnginesSound` (`self.EngineStart_Sound`))
              (`KismetSystemLibrary.Delay` (`self.PowerTime`))
              (`self.GravityEngineActivate` false))))
        (:`then_1`
          (goto _label_2 :!via `Reset`)))
      (else
        (`|ExecutionSequence`
          (:`then_0`
            (`/Engine/EditorBlueprintResources/StandardMacros.DoOnce` false :!label _label_2
              (:`Completed`
                (`self.SetComponentTickEnabled` false)
                (if (`self.GravityEnginesActive`)
                  (set `self.IsCooldown` true)
                  (`self.GravityEngine_Cooldown` (`self.Cooldown`))
                  (`self.ResetEffects`)
                  (set `self.GravityEnginesActive` false)
                  (`self.SetActive` (`self.Particle_Backward`) false false)
                  (`self.SetActive` (`self.Particle_Forward`) false false)
                  (`self.SetActive` (`self.Particle_Right`) false false)
                  (`self.SetActive` (`self.Particle_Left`) false false)
                  (`self.PlayGravityEnginesSound` (`self.EngineEnd_Sound`))
                  (`KismetSystemLibrary.Delay` (`self.Cooldown`))
                  (set `self.IsCooldown` false)))))
          (:`then_1`
            (goto _label :!via `Reset`)))))))

(event `ResetEffects`
  (bind _returnvalue (> (`self.AxisMoveRight`) 0.0))
  (bind _returnvalue_2 (> (`self.AxisMoveForward`) 0.0))
  (bind _returnvalue_3 (not _returnvalue_2))
  (bind _returnvalue_4 (not _returnvalue))
  ;[1 1 1] GravityEngines Physics
  (`self.GravityEngineActive_Fwd` false)
  (`self.GravityEngineActive_Right` false)
  (`|ExecutionSequence`
    (:`then_0`
      (goto _label_3 :!via `Reset`))
    (:`then_1`
      (goto _label_4 :!via `Reset`))
    (:`then_2`
      (goto _label_5 :!via `Reset`))
    (:`then_3`
      (goto _label_6 :!via `Reset`))))

(event `self.ReceiveTick`
  (params (DeltaSeconds :type "Float (single-precision)"))
  (bind _returnvalue (> (`self.AxisMoveRight`) 0.0))
  (bind _returnvalue_2 (> (`self.AxisMoveForward`) 0.0))
  (bind _returnvalue_3 (not _returnvalue_2))
  (bind _returnvalue_4 (not _returnvalue))
  ;[1 1 1] GravityEngines Physics
  (`PrimitiveComponent.SetPhysicsAngularVelocityInDegrees` (`WheeledVehiclePawn.Mesh` (`self.Car`)) (* (`KismetMathLibrary.Normal` (+ (* (`SceneComponent.GetForwardVector` (`WheeledVehiclePawn.Mesh` (`self.Car`))) (* (`self.AxisMoveRight`) -1.0)) (* (`SceneComponent.GetRightVector` (`WheeledVehiclePawn.Mesh` (`self.Car`))) (`self.AxisMoveForward`)))) (select `bool` (`/Game/Interaction/Blueprints/Pawn/Car/Components/BP_Nitro_Comp.NitroIsActive?` (`/Game/Interaction/Blueprints/Pawn/Car/Pawn_ChaosCar.Nitro` (`self.Car`))) :`false` (`self.EnginePower`) :`true` (`self.EnginePowerWithNitro`))) true (`self.BoneNameForForce`))
  (`|ExecutionSequence`
    (:`then_0`
      (if (!= (`self.AxisMoveForward`) 0.0)
        (`|ExecutionSequence`
          (:`then_0`
            (`/Engine/EditorBlueprintResources/StandardMacros.DoOnce` false :!label _label_3
              (:`Completed`
                (`self.SetActive` (`self.Particle_Forward`) _returnvalue_3 false)
                (`self.SetActive` (`self.Particle_Backward`) _returnvalue_2 false)
                (`self.GravityEngineActive_Fwd` _returnvalue_3 true))))
          (:`then_1`
            (goto _label_4 :!via `Reset`)))
        (else
          (`|ExecutionSequence`
            (:`then_0`
              (`/Engine/EditorBlueprintResources/StandardMacros.DoOnce` false :!label _label_4
                (:`Completed`
                  (`self.SetActive` (`self.Particle_Backward`) false false)
                  (`self.SetActive` (`self.Particle_Forward`) false false)
                  (`self.GravityEngineActive_Fwd` false))))
            (:`then_1`
              (goto _label_3 :!via `Reset`))))))
    (:`then_1`
      (if (!= (`self.AxisMoveRight`) 0.0)
        (`|ExecutionSequence`
          (:`then_0`
            (`/Engine/EditorBlueprintResources/StandardMacros.DoOnce` false :!label _label_5
              (:`Completed`
                (`self.SetActive` (`self.Particle_Right`) _returnvalue_4 false)
                (`self.SetActive` (`self.Particle_Left`) _returnvalue false)
                (`self.GravityEngineActive_Right` _returnvalue_4 true))))
          (:`then_1`
            (goto _label_6 :!via `Reset`)))
        (else
          (`|ExecutionSequence`
            (:`then_0`
              (`/Engine/EditorBlueprintResources/StandardMacros.DoOnce` false :!label _label_6
                (:`Completed`
                  (`self.SetActive` (`self.Particle_Right`) false false)
                  (`self.SetActive` (`self.Particle_Left`) false false)
                  (`self.GravityEngineActive_Right` false))))
            (:`then_1`
              (goto _label_5 :!via `Reset`))))))))

(fn `PlayGravityEnginesSound`
  (params (Sound :type "SoundBase Object Reference"))
  (bind _sound (`self.Sound`))
  (`AudioComponent.Stop` _sound)
  (`AudioComponent.SetSound` _sound Sound)
  (`AudioComponent.Play` _sound 0.0))