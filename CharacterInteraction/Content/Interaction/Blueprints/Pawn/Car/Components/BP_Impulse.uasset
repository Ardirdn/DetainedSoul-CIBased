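; Car component for Pawn_ChaosCar that provides a chargeable shockwave ability with cooldown.
; BeginPlay attaches the particle, sound and optional impulser mesh with a dynamic glow material.
; A looping timer builds power, updating the glow and broadcasting the charge level.
; On release above a threshold, power scales the effect and radial damage radius, adds camera shake and can make the car jump; weaker releases play a cancel sound.
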(event `self.ReceiveBeginPlay`
  ;[1 1 1] Initialization
  (bind _aspawn_chaos_car (cast `/Game/Interaction/Blueprints/Pawn/Car/Pawn_ChaosCar` (`self.GetOwner`))
    (:`then`
      (set `self.Car` _aspawn_chaos_car)
      (bind _returnvalue (`GameplayStatics.SpawnEmitterAttached` (`self.ImpulseParticle`) (`WheeledVehiclePawn.Mesh` (`self.Car`)) "None" (`self.RelativeLocation`) (struct) (1.0 1.0 1.0) "KeepRelativeOffset" false))
      (bind _output_get (set `self.Particle` _returnvalue))
      (`self.SetActive` _output_get false false)
      (bind _returnvalue_2 (`GameplayStatics.SpawnSoundAttached` (`self.ImpulseSound`) (`WheeledVehiclePawn.Mesh` (`self.Car`)) "None" (`self.RelativeLocation`) (struct) "KeepRelativeOffset" false 1.0 1.0 0.0 null null false))
      (bind _output_get_2 (set `self.Sound` _returnvalue_2))
      (`AudioComponent.Stop` _output_get_2)
      (`/Engine/EditorBlueprintResources/StandardMacros.IsValid` (`self.ImpulserMesh`)
        (:`Is Valid`
          (bind _returnvalue_3 (`|SpawnActorFromClass` "/Script/Engine.StaticMeshActor" (`KismetMathLibrary.MakeTransform` (0.0 0.0 0.0)) "AlwaysSpawn" "OverrideRootScale" (`self.Car`) null))
          (set `self.ImpulserMesh_Ref` _returnvalue_3)
          (`PrimitiveComponent.SetCollisionResponseToChannel` (`StaticMeshActor.StaticMeshComponent` (`self.ImpulserMesh_Ref`)) "ECC_GameTraceChannel5" "ECR_Ignore")
          (`StaticMeshActor.SetMobility` (`self.ImpulserMesh_Ref`) "Movable")
          (`StaticMeshComponent.SetStaticMesh` (`StaticMeshActor.StaticMeshComponent` (`self.ImpulserMesh_Ref`)) (`self.ImpulserMesh`))
          (`Actor.K2_AttachToComponent` (`self.ImpulserMesh_Ref`) (`WheeledVehiclePawn.Mesh` (`self.Car`)) "None" "KeepRelative" "KeepRelative" "KeepRelative" true)
          (`SceneComponent.K2_SetRelativeTransform` (`StaticMeshActor.StaticMeshComponent` (`self.ImpulserMesh_Ref`)) (`KismetMathLibrary.MakeTransform` (0.0 0.0 0.0)) false false)
          (`/Engine/EditorBlueprintResources/StandardMacros.IsValid` (`self.ImpulseMeshMaterial`)
            (:`Is Valid`
              (bind _returnvalue_4 (`PrimitiveComponent.CreateDynamicMaterialInstance` (`StaticMeshActor.StaticMeshComponent` (`self.ImpulserMesh_Ref`)) (`self.MaterialIndex`) (`self.ImpulseMeshMaterial`) "None"))
              (bind _output_get_3 (set `self.Material` _returnvalue_4))
              (`MaterialInstanceDynamic.SetVectorParameterValue` _output_get_3 "ImpulseEmColor" (`self.ImpulseEmissiveColor`)))))))
    (:`CastFailed`
      (`KismetSystemLibrary.PrintString` "(Impulse System) Owner actor is not a car"))))

(event `StartChargeImpulse`
  ;[1 1 1] Start charging
  (if (`self.ImpulseReady`)
    (bind _returnvalue (`KismetSystemLibrary.K2_SetTimer` null "ChargeImpulse" (`self.PowerTime`) true))
    (set `self.Timer_ChargeImpulse` _returnvalue)
    ;[1 1 1] Play charge sound
    (`self.PlayImpulseSound` (`self.ChargeSound`))))

(event `StopChargeImpulse`
  (bind _car (`self.Car`))
  (bind _currentradius (`self.CurrentRadius`))
  ;[1 1 1] Active Impulse
  (`KismetSystemLibrary.K2_ClearAndInvalidateTimerHandle` (`self.Timer_ChargeImpulse`))
  (`self.CurrentImpulse_Power` 0.0)
  (if (> (`self.CurrentImpulsePower`) (`self.MinPulseThreshold`))
    (set `self.ImpulseReady` false)
    (`self.ImpulseActive` (`self.CoolDown_Time`))
    (set `self.CurrentRadius` (`KismetMathLibrary.MapRangeClamped` (`self.CurrentImpulsePower`) 0.0 1.0 (`self.ImpulseRadius_Min`) (`self.ImpulseRadius_Max`)))
    (`ParticleSystemComponent.SetVectorParameter` (`self.Particle`) "ImpulseRadius" (`KismetMathLibrary.MakeVector` _currentradius _currentradius _currentradius))
    ;[1 1 1] Impulse Effects
    (`self.SetActive` (`self.Particle`) true true)
    (`/Game/Interaction/Blueprints/CharacterInteraction_FunctionLibrary.RadialDamage` (`|MakeArray` _car (`/Game/Interaction/Blueprints/Pawn/Car/Pawn_ChaosCar.CharacterDriver` _car) :!type "Actor Object Reference") (+ (`SceneComponent.K2_GetComponentLocation` (`WheeledVehiclePawn.Mesh` _car)) (`self.RelativeLocation`)) (* (`self.CurrentRadius`) 10.0) (`|MakeArray` "ObjectTypeQuery2" "ObjectTypeQuery3" "ObjectTypeQuery4" "ObjectTypeQuery5" :!type "EObjectTypeQuery Enum") (`self.Car`) (`self.DamageType`) (`self.DoFullDamage`) (`self.ImpulseDamage`))
    (`PlayerCameraManager.StartCameraShake` :`self` (`PlayerController.PlayerCameraManager` (`GameplayStatics.GetPlayerController` 0)) :`ShakeClass` (`self.CameraShake`) :`Scale` (`self.CameraShakeScale`))
    (`self.PlayImpulseSound` (`self.ImpulseSound`))
    ;[1 1 1] Reset glow effect
    (`|ExecutionSequence`
      (:`then_0`
        ;[1 1 1] Car jump impulse
        (if (> (`self.CurrentImpulsePower`) (`self.MinJumpThreshold`))
          (`PrimitiveComponent.AddImpulse` (`WheeledVehiclePawn.Mesh` (`self.Car`)) (* (`self.JumpVector`) (`KismetMathLibrary.MapRangeClamped` (`self.CurrentImpulsePower`) 0.0 1.0 (`self.CarJumpImpulse_Min`) (`self.CarJumpImpulse_Max`))) "None" true))
        (set `self.CurrentImpulsePower` 0.0)
        ;[1 1 1] Cooldown
        (`KismetSystemLibrary.Delay` (`self.CoolDown_Time`))
        (set `self.ImpulseReady` true))
      (:`then_1`
        (`/Engine/EditorBlueprintResources/StandardMacros.IsValid` (`self.Material`)
          (:`Is Valid`
            (`MaterialInstanceDynamic.SetScalarParameterValue` (`self.Material`) "ImpulseEmPercent" 200.0)
            (`KismetSystemLibrary.Delay` 0.3)
            (`MaterialInstanceDynamic.SetScalarParameterValue` (`self.Material`) "ImpulseEmPercent" 0.0)))))
    (else
      (`self.PlayImpulseSound` (`self.CancelSound`)))))

(fn `ChargeImpulse`
  (bind _output_get (set `self.CurrentImpulsePower` (+ (`self.CurrentImpulsePower`) (`self.ImpulseCharge_PerTime`))))
  (if (> _output_get 1.0)
    (set `self.CurrentImpulsePower` 1.0)
    (`self.CurrentImpulse_Power` 1.0)
    (`KismetSystemLibrary.K2_ClearAndInvalidateTimerHandle` (`self.Timer_ChargeImpulse`))
    (else
      (`self.CurrentImpulse_Power` (`self.CurrentImpulsePower`))
      (`/Engine/EditorBlueprintResources/StandardMacros.IsValid` (`self.Material`)
        (:`Is Valid`
          (`MaterialInstanceDynamic.SetScalarParameterValue` (`self.Material`) "ImpulseEmPercent" (`self.CurrentImpulsePower`)))))))

(fn `PlayImpulseSound`
  (params (Sound :type "SoundBase Object Reference"))
  (bind _sound (`self.Sound`))
  (`AudioComponent.Stop` _sound)
  (`AudioComponent.SetSound` _sound Sound)
  (`AudioComponent.Play` _sound 0.0))