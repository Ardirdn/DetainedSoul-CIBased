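; Car component that drives headlights, brake, reverse and turn signal lights on a Pawn_ChaosCar.
; On BeginPlay it creates a dynamic material on the car mesh, sets light colours and caches the two front spot lights.
; Events set emissive strengths on that material; the front switch also cycles the spot lights through off, dipped and high beam, with a click sound.
; Optional turn signals blink through looping timers and FlipFlops.
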(event `self.ReceiveBeginPlay`
  ;[1 1 1] Begind play Initialization
  (bind _output_get (set `self.Car` (cast `/Game/Interaction/Blueprints/Pawn/Car/Pawn_ChaosCar` (`self.GetOwner`) :!pure true)))
  (bind _returnvalue (`PrimitiveComponent.CreateDynamicMaterialInstance` (`WheeledVehiclePawn.Mesh` _output_get) (`self.MaterialIndex`) (`self.Material`) "None"))
  (set `self.CurrentMaterial` _returnvalue)
  (`self.SetLightsColor`)
  (`self.AddFrontSpotLights`))

(event `FrontLightSwitch`
  ;[1 1 1] Front Lights
  (bind _result (`/Engine/EditorBlueprintResources/StandardMacros.IncrementInt` (`self.FrontLightStateIndex`))
    (:`  `
      (if (> _result 2)
        (set `self.FrontLightStateIndex` 0))
      (switch `string` (`KismetStringLibrary.Conv_IntToString` (`self.FrontLightStateIndex`))
        (:`0`
          (`MaterialInstanceDynamic.SetScalarParameterValue` (`self.CurrentMaterial`) "FrontLight_Strength" 0.0)
          (`SceneComponent.SetVisibility` (`self.RightFrontLight`) false false)
          (`SceneComponent.SetVisibility` (`self.LeftFrontLight`) false false))
        (:`1`
          (`MaterialInstanceDynamic.SetScalarParameterValue` (`self.CurrentMaterial`) "FrontLight_Strength" (`self.DippedHeadlights_Em`))
          (`SceneComponent.SetVisibility` (`self.RightFrontLight`) true false)
          (`SceneComponent.SetVisibility` (`self.LeftFrontLight`) true false)
          (`LightComponent.SetIntensity` (`self.RightFrontLight`) (`self.DippedHeadlights`))
          (`LightComponent.SetIntensity` (`self.LeftFrontLight`) (`self.DippedHeadlights`))
          (`PointLightComponent.SetAttenuationRadius` (`self.RightFrontLight`) (`self.DippedHeadlights_Radius`))
          (`PointLightComponent.SetAttenuationRadius` (`self.LeftFrontLight`) (`self.DippedHeadlights_Radius`)))
        (:`2`
          (`MaterialInstanceDynamic.SetScalarParameterValue` (`self.CurrentMaterial`) "FrontLight_Strength" (`self.HighBeamHeadlights_Em`))
          (`SceneComponent.SetVisibility` (`self.RightFrontLight`) true false)
          (`SceneComponent.SetVisibility` (`self.LeftFrontLight`) true false)
          (`LightComponent.SetIntensity` (`self.RightFrontLight`) (`self.HighBeamHeadlights`))
          (`LightComponent.SetIntensity` (`self.LeftFrontLight`) (`self.HighBeamHeadlights`))
          (`PointLightComponent.SetAttenuationRadius` (`self.RightFrontLight`) (`self.HighBeamHeadlights_Radius`))
          (`PointLightComponent.SetAttenuationRadius` (`self.LeftFrontLight`) (`self.HighBeamHeadlights_Radius`))))
      (`GameplayStatics.PlaySound2D` (`self.Sound_LightSwitch`) 1.0 1.0 0.0 null null))))

(event `BrakeLights`
  (params (Active :type Boolean))
  ;[1 1 1] Brake Lights
  (`MaterialInstanceDynamic.SetScalarParameterValue` (`self.CurrentMaterial`) "BrakeLight_Strength" (select `bool` Active :`true` (`self.BrakeLights_Em`))))

(event `TurnSignalsLeft`
  (params (Active :type Boolean))
  ;[1 1 1] Turn Signals Left
  (if (`self.UseTurnSignals`)
    (if Active
      (bind _returnvalue (`KismetSystemLibrary.K2_SetTimerDelegate` (delegate `TurnSignalsLeftFlash`) (`self.FlashDelay`) true))
      (set `self.Timer_TurnLeftFlash` _returnvalue)
      (else
        (`KismetSystemLibrary.K2_ClearAndInvalidateTimerHandle` (`self.Timer_TurnLeftFlash`))
        (`MaterialInstanceDynamic.SetScalarParameterValue` (`self.CurrentMaterial`) "TurnSignalsLeft_Strength" 0.0 :!label _label)))))

(event `TurnSignalsRight`
  (params (Active :type Boolean))
  ;[1 1 1] Turn Signals Right
  (if (`self.UseTurnSignals`)
    (if Active
      (bind _returnvalue (`KismetSystemLibrary.K2_SetTimerDelegate` (delegate `TurnSignalsRightFlash`) (`self.FlashDelay`) true))
      (set `self.Timer_TurnRightFlash` _returnvalue)
      (else
        (`KismetSystemLibrary.K2_ClearAndInvalidateTimerHandle` (`self.Timer_TurnRightFlash`))
        (`MaterialInstanceDynamic.SetScalarParameterValue` (`self.CurrentMaterial`) "TurnSignalsRight_Strength" 0.0 :!label _label_2)))))

(event `TurnSignalsLeftFlash`
  ;[1 1 1] Turn Signals Left
  (`/Engine/EditorBlueprintResources/StandardMacros.FlipFlop`
    (:`A`
      (`MaterialInstanceDynamic.SetScalarParameterValue` (`self.CurrentMaterial`) "TurnSignalsLeft_Strength" (`self.TurnSignals_Em`)))
    (:`B`
      (goto _label))))

(event `TurnSignalsRightFlash`
  ;[1 1 1] Turn Signals Right
  (`/Engine/EditorBlueprintResources/StandardMacros.FlipFlop`
    (:`A`
      (`MaterialInstanceDynamic.SetScalarParameterValue` (`self.CurrentMaterial`) "TurnSignalsRight_Strength" (`self.TurnSignals_Em`)))
    (:`B`
      (goto _label_2))))

(event `ReverseLights`
  (params (Active :type Boolean))
  ;[1 1 1] Reverse Lights
  (`MaterialInstanceDynamic.SetScalarParameterValue` (`self.CurrentMaterial`) "ReverseLight_Strength" (select `bool` Active :`true` (`self.ReverseLight_Em`))))

(fn `AddFrontSpotLights`
  (set `self.RightFrontLight` (`/Game/Interaction/Blueprints/Pawn/Car/Pawn_ChaosCar.FrontLight_R` (`self.Car`)))
  (`LightComponent.SetLightColor` (`self.RightFrontLight`) (`self.LightColor`) true)
  (set `self.LeftFrontLight` (`/Game/Interaction/Blueprints/Pawn/Car/Pawn_ChaosCar.FrontLight_L` (`self.Car`)))
  (`LightComponent.SetLightColor` (`self.LeftFrontLight`) (`self.LightColor`) true))

(fn `SetLightsColor`
  (`MaterialInstanceDynamic.SetVectorParameterValue` (`self.CurrentMaterial`) "FrontLight_Color" (`self.FrontLightsColor`))
  (`MaterialInstanceDynamic.SetVectorParameterValue` (`self.CurrentMaterial`) "BrakeLight_Color" (`self.BrakeLightsColor`))
  (`MaterialInstanceDynamic.SetVectorParameterValue` (`self.CurrentMaterial`) "ReverseLight_Color" (`self.ReverseLightsColor`))
  (`MaterialInstanceDynamic.SetVectorParameterValue` (`self.CurrentMaterial`) "TurnSignals_Color" (`self.TurnSignalsColor`)))