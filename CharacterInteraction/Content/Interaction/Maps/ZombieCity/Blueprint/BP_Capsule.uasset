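; BP_Capsule is a scripted capsule in the ZombieCity map, with a start scene where the player exits it and a separate end scene.
; StartScene flags the player's Interaction component, plays a slot montage and snaps the character to the capsule's CharacterPlace socket alongside the capsule animation.
; Timed delays then switch to idle, make the interaction interruptible, kill the light and remove droplet particles.
; End_Scene plays the closing animation while toggling the light and jet effect.
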(event `StartScene`
  (bind _capsule (`self.Capsule`))
  (bind _output_get (set `self.Player` (cast `Character` (`GameplayStatics.GetPlayerPawn` 0) :!pure true)))
  (bind (_hud _inventory _interaction) (message `/Game/Interaction/Blueprints/Pawn/Player/StatusInterface.GetComponents` _output_get))
  (`/Game/Interaction/Blueprints/Pawn/Player/Components/BP_Interaction.SetIsInteraction` _interaction true)
  (`AnimInstance.PlaySlotAnimationAsDynamicMontage` (`SkeletalMeshComponent.GetAnimInstance` (`Character.Mesh` _output_get)) "/Game/Interaction/Animations/Cutscene/A_CS_StartExitCapsule.A_CS_StartExitCapsule" "Interaction" 0.0 0.25 1.0 1 -1.0 0.0)
  (`self.K2_SetActorTransform` (`self.Player`) (`SceneComponent.GetSocketTransform` (`self.Capsule`) "CharacterPlace" "RTS_World") false true)
  (`SkeletalMeshComponent.PlayAnimation` _capsule "/Game/Interaction/Maps/ZombieCity/Meshes/Capsule/Animations/A_Capsule_Start.A_Capsule_Start" false)
  (`|ExecutionSequence`
    (:`then_0`
      (`KismetSystemLibrary.Delay` 17.4)
      (`SkeletalMeshComponent.PlayAnimation` _capsule "/Game/Interaction/Maps/ZombieCity/Meshes/Capsule/Animations/A_Capsule_Idle.A_Capsule_Idle" true)
      (bind (_hud_2 _inventory_2 _interaction_2) (message `/Game/Interaction/Blueprints/Pawn/Player/StatusInterface.GetComponents` (`self.Player`)))
      (`/Game/Interaction/Blueprints/Pawn/Player/Components/BP_Interaction.SetCanInterruptInteract` _interaction_2 true))
    (:`then_1`
      (`KismetSystemLibrary.Delay` 15.7)
      (`LightComponent.SetIntensity` (`self.PointLight`) 0.0)
      (`KismetSystemLibrary.Delay` 7.0)
      (`ActorComponent.SetActive` (`self.P_Droplets_01`) false true)
      (`ActorComponent.SetActive` (`self.P_Droplets_05`) false true)
      (`ActorComponent.SetActive` (`self.P_Droplets_04`) false true)
      (`ActorComponent.SetActive` (`self.P_Droplets_03`) false true)
      (`ActorComponent.SetActive` (`self.P_Droplets_02`) false true)
      (`KismetSystemLibrary.Delay` 3.0)
      (`ActorComponent.K2_DestroyComponent` (`self.P_Droplets_02`))
      (`ActorComponent.K2_DestroyComponent` (`self.P_Droplets_03`))
      (`ActorComponent.K2_DestroyComponent` (`self.P_Droplets_04`))
      (`ActorComponent.K2_DestroyComponent` (`self.P_Droplets_01`))
      (`ActorComponent.K2_DestroyComponent` (`self.P_Droplets_05`)))))

(event `End_Scene`
  (`SkeletalMeshComponent.PlayAnimation` (`self.Capsule`) "/Game/Interaction/Maps/ZombieCity/Meshes/Capsule/Animations/A_Capsule_End.A_Capsule_End" false)
  (`LightComponent.SetIntensity` (`self.PointLight`) 0.0)
  (`|ExecutionSequence`
    (:`then_0`
      (`KismetSystemLibrary.Delay` 0.8)
      (`ActorComponent.SetActive` (`self.P_BlossomJet`) false false))
    (:`then_1`
      (`KismetSystemLibrary.Delay` 2.0)
      (`ActorComponent.SetActive` (`self.P_BlossomJet`) true false)
      (`LightComponent.SetIntensity` (`self.PointLight`) 100.0))))

(fn `UserConstructionScript`)